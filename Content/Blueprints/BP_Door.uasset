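; BP_Door is an interactable door that responds only to the key assigned to it.
; OnInteract checks the interacting character's HeldItem, casts it to BP_Key and compares that key's Unlocks reference to this door.
; A match only prints an "Open Door" debug message; the door has no opening logic, and its default events are disabled stubs.
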(fn `OnInteract`
  (params (Character :type "/Game/Blueprints/BP_Char Object Reference"))
  (bind _helditem (`/Game/Blueprints/BP_Char.HeldItem` Character))
  (if (`KismetSystemLibrary.IsValid` _helditem)
    (bind _asbp_key (cast `/Game/Blueprints/BP_Key` _helditem))
    (if (== (`/Game/Blueprints/BP_Key.Unlocks` _asbp_key) self)
      (`KismetSystemLibrary.PrintString` "Open Door"))))

(fn `UserConstructionScript`
  (`parent.UserConstructionScript`))
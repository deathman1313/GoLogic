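; BP_Cage is an interactable cage whose hinged door opens only with its matching key.
; OnInteract checks that the character's held item is a BP_Key whose Unlocks reference points to this cage, then destroys it and clears the held item.
; OpenDoor plays the SwingAngle timeline, lerping the Hinge's relative yaw to swing the door open.
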(event `OpenDoor`
  (bind (_direction _swing) (`Timeline|SwingAngle`)
    (:`Update`
      (`SceneComponent.K2_SetRelativeRotation` (`self.Hinge`) (`KismetMathLibrary.MakeRotator` 0.0 0.0 (`KismetMathLibrary.Lerp` 0.0 110.0 _swing)) false false))))

(fn `OnInteract`
  (params (Character :type "/Game/Blueprints/BP_Char Object Reference"))
  (bind _helditem (`/Game/Blueprints/BP_Char.HeldItem` Character))
  (if (`KismetSystemLibrary.IsValid` _helditem)
    (bind _asbp_key (cast `/Game/Blueprints/BP_Key` _helditem))
    (if (== (`/Game/Blueprints/BP_Key.Unlocks` _asbp_key) self)
      (`self.K2_DestroyActor` _helditem)
      (set `/Game/Blueprints/BP_Char.HeldItem` null Character)
      (`self.OpenDoor`))))

(fn `UserConstructionScript`
  (`parent.UserConstructionScript`))
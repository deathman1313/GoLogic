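; BP_Pickup is an interactable item that characters can pick up and hold.
; OnInteract ignores items already held and blocks BP_CharSmall from taking items flagged IsLarge, while other characters can take any size.
; PickupItem requires the character to have no valid HeldItem, then records itself there, attaches to the mesh's HeldItem socket and sets Held.
; It contains no drop logic.
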(fn `OnInteract`
  (params (Character :type "/Game/Blueprints/BP_Char Object Reference"))
  (if (not (`self.Held`))
    (cast `/Game/Blueprints/BP_CharSmall` Character
      (:`then`
        (if (not (`self.IsLarge`))
          (`self.Pickup Item` Character :!label _label)))
      (:`CastFailed`
        (goto _label)))))

(fn `Pickup Item`
  (params (Character :type "/Game/Blueprints/BP_Char Object Reference"))
  (if (not (`KismetSystemLibrary.IsValid` (`/Game/Blueprints/BP_Char.HeldItem` Character)))
    (set `/Game/Blueprints/BP_Char.HeldItem` self Character)
    (`self.K2_AttachToComponent` self (`Character.Mesh` Character) "HeldItem" "KeepRelative" "KeepRelative" "KeepRelative" true)
    (set `self.Held` true)))

(fn `UserConstructionScript`
  (`parent.UserConstructionScript`))
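; BP_Interactable is an interactable object that characters can pick up and that shows its name when hovered.
; Hover events write or clear the object name in the HUD's select text through BP_GM1.
; Interact blocks BP_CharSmall from taking objects flagged IsLarge, while other characters can take any.
; PickupItem attaches to the character mesh's HeldItem socket if HeldItem is invalid, but never sets that variable.
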(event `/Game/Blueprints/BPI_Interact.Interact`
  (params (Character :type "/Game/Blueprints/BP_Char Object Reference"))
  (cast `/Game/Blueprints/BP_CharSmall` Character
    (:`then`
      (if (not (`self.IsLarge`))
        (`self.PickupItem` Character :!label _label)))
    (:`CastFailed`
      (goto _label))))

(event `/Game/Blueprints/BPI_Interact.Hovered`
  (params (Character :type "/Game/Blueprints/BP_Char Object Reference"))
  (bind _asbp_gm1 (cast `/Game/Blueprints/BP_GM1` (`GameplayStatics.GetGameMode`)))
  (`TextBlock.SetText` (`/Game/UI/WBP_HUD.Txt_SelectText` (`/Game/Blueprints/BP_GM1.HUD` _asbp_gm1)) (`self.ObjectName`)))

(event `/Game/Blueprints/BPI_Interact.Unhovered`
  (params (Character :type "/Game/Blueprints/BP_Char Object Reference"))
  (bind _asbp_gm1 (cast `/Game/Blueprints/BP_GM1` (`GameplayStatics.GetGameMode`)))
  (`TextBlock.SetText` (`/Game/UI/WBP_HUD.Txt_SelectText` (`/Game/Blueprints/BP_GM1.HUD` _asbp_gm1)) ""))

(fn `PickupItem`
  (params (Character :type "/Game/Blueprints/BP_Char Object Reference"))
  (if (not (`KismetSystemLibrary.IsValid` (`/Game/Blueprints/BP_Char.HeldItem` Character)))
    (`self.K2_AttachToComponent` self (`Character.Mesh` Character) "HeldItem" "KeepRelative" "KeepRelative" "KeepRelative" true)))

(fn `UserConstructionScript`)